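; Player controller for an idle monster clicker that owns the main UI and spawns enemies, items and click feedback.
; On BeginPlay it caches the pawn, shows the main widget, sets a custom cursor, builds shop cards from the item DataTable and adds the first level button.
; Shop buy buttons are recolored and enabled by comparing item cost to the pawn's coins.
; Floating text also triggers a hit effect at the deprojected mouse position.
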(event Custom|SpawnEnemy
  (params (Enemy :type Actor%20Class%20Reference) (SpawnTransform :type Transform))
  (bind _returnvalue (Game|SpawnActorfromClass Enemy SpawnTransform "AdjustIfPossibleButAlwaysSpawn" "MultiplyWithRoot" 0 0))
  (bind _enemy (Class|BPIEnemy|GetEnemyRef(Message) _returnvalue))
  (Variables|Default|SetSpawnedEnemy _enemy))

(event Custom|SpawnHitEffect
  (Game|SpawnActorfromClass "/Game/Dynamic/Blueprints/BP_HitEffect.BP_HitEffect_C" (Math|Conversions|ToTransform(Vector) (- (.WorldLocation (Game|Player|ConvertMouseLocationToWorldSpace)) "0.000000,1.000000,0.000000")) "AlwaysSpawn" "MultiplyWithRoot" 0 0))

(event Custom|SpawnFloatingText
  (params (SpawnLocation :type Vector) (Text :type String))
  (bind (_x _y _z) (Math|Vector|BreakVector SpawnLocation))
  (Game|SpawnActorfromClass "/Game/Dynamic/Blueprints/BP_FloatingText.BP_FloatingText_C" (Math|Transform|MakeTransform (Math|Vector|MakeVector _x 1.0 (+ _z 18.0))) "AlwaysSpawn" "MultiplyWithRoot" 0 Text 0)
  (CallFunction|SpawnHitEffect))

(event Custom|ShowHideWidget
  (params (Widgets :type E_GameWidgets%20Enum :default "NewEnumerator0") (bShow :type Boolean))
  (if bShow
    (CallFunction|ShowWidget Widgets)
    (else
      (CallFunction|HideWidget Widgets))))

(event Custom|CreateShopItemCards
  (Utilities|Array|Clear (Variables|Default|GetShopItemCards))
  (bind _outrownames (DataTable|GetDataTableRowNames "/Game/Dynamic/Blueprints/DataTables/DT_ItemInfo.DT_ItemInfo"))
  (for _array_element _outrownames
    (bind _returnvalue (UserInterface|CreateWidget "/Game/Dynamic/UI/WB_ShopItemCard.WB_ShopItemCard_C" 0 (CallFunction|GetItemInfo (Utilities|String|ToString(Name) _array_element))))
    (Utilities|Array|Add (Variables|Default|GetShopItemCards) _returnvalue))
  (CallFunction|DisplayShopItemCards)
  (CallFunction|UpdateShopItemBuyTextColor))

(event Custom|DisplayShopItemCards
  (Widget|Panel|ClearChildren (Variables|/Game/Dynamic/UI/WB_MainUI.WB_MainUI_C|GetVB_ItemList (Variables|Default|GetWB_Main)))
  (for _array_element (Variables|Default|GetShopItemCards)
    (Class|VerticalBox|AddChildtoVerticalBox (Variables|/Game/Dynamic/UI/WB_MainUI.WB_MainUI_C|GetVB_ItemList (Variables|Default|GetWB_Main)) _array_element)))

(event Custom|SpawnItem
  (params (Item :type Actor%20Class%20Reference) (Location :type Vector))
  (Game|SpawnActorfromClass Item (Math|Transform|MakeTransform Location) "Undefined" "MultiplyWithRoot" 0 0))

(event Custom|InitializePlayer
  (bind _returnvalue (UserInterface|CreateWidget "/Game/Dynamic/UI/WB_ShopToolTip.WB_ShopToolTip_C"))
  (Variables|Default|SetShopToolTip _returnvalue)
  (bind _returnvalue_2 (UserInterface|CreateWidget "/Game/Dynamic/UI/WB_MouseCursor.WB_MouseCursor_C"))
  (bind _output_get (Variables|Default|SetMouseCursor _returnvalue_2))
  (Class|PlayerController|SetMouseCursorWidget "Default" _output_get))

(event Custom|AddLevelButtonUI
  (params (Level :type Integer))
  (bind _returnvalue (UserInterface|CreateWidget "/Game/Dynamic/UI/WB_LevelCard.WB_LevelCard_C" 0 Level))
  (Class|VerticalBox|AddChildtoVerticalBox (Variables|/Game/Dynamic/UI/WB_MainUI.WB_MainUI_C|GetVB_LevelList (Variables|Default|GetWB_Main)) _returnvalue))

(event EventBeginPlay
  (bind _player (Class|BPIPlayer|GetPlayerRef(Message) (Game|GetPlayerCharacter 0)))
  (Variables|Default|SetPlayerPawn _player)
  (CallFunction|ShowHideWidget "NewEnumerator0" true)
  (CallFunction|InitializePlayer)
  (CallFunction|CreateShopItemCards)
  (CallFunction|AddLevelButtonUI 1))

(fn ConstructionScript)

(fn ShowWidget
  (params (Widget :type E_GameWidgets%20Enum :default "NewEnumerator0"))
  (switch Utilities|FlowControl|Switch|SwitchonE_GameWidgets Widget
    (:NewEnumerator0
      (Variables|Default|GetWB_Main
        (:then
          _)
        (:else
          (bind _returnvalue (UserInterface|CreateWidget "/Game/Dynamic/UI/WB_MainUI.WB_MainUI_C"))
          (bind _output_get (Variables|Default|SetWB_Main _returnvalue))))
      (UserInterface|Viewport|AddtoViewport _output_get 0))))

(fn HideWidget
  (params (Widget :type E_GameWidgets%20Enum :default "NewEnumerator0"))
  (switch Utilities|FlowControl|Switch|SwitchonE_GameWidgets Widget
    (:NewEnumerator0
      (bind _wb_main (Variables|Default|GetWB_Main)
        (:then
          (Widget|RemovefromParent _wb_main))
        (:else)))))

(fn UpdateShopItemBuyTextColor
  (for _array_element (Variables|Default|GetShopItemCards)
    (Appearance|SetColorandOpacity (Variables|/Game/Dynamic/UI/WB_ShopItemCard.WB_ShopItemCard_C|GetT_Buy _array_element) (Utilities|Struct|MakeSlateColor (Math|Color|SelectColor "(R=1.000000,G=0.000000,B=0.011765,A=1.000000)" "(R=1.000000,G=0.290196,B=0.000000,A=1.000000)" (> (Default|GetItemCost (Variables|Default|GetPlayerPawn) (Variables|/Game/Dynamic/UI/WB_ShopItemCard.WB_ShopItemCard_C|GetItemInfo _array_element)) (Variables|/Game/Dynamic/Blueprints/BP_Player.BP_Player_C|GetAmountOfCoins (Variables|Default|GetPlayerPawn))))) :!class /Script/UMG.TextBlock)
    (Widget|SetIsEnabled (Variables|/Game/Dynamic/UI/WB_ShopItemCard.WB_ShopItemCard_C|GetBTN_Buy _array_element) (select (> (Default|GetItemCost (Variables|Default|GetPlayerPawn) (Variables|/Game/Dynamic/UI/WB_ShopItemCard.WB_ShopItemCard_C|GetItemInfo _array_element)) (Variables|/Game/Dynamic/Blueprints/BP_Player.BP_Player_C|GetAmountOfCoins (Variables|Default|GetPlayerPawn))) false true))))

(fn GetPlayerControlRef
  (return self))