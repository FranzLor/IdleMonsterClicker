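; Player Blueprint for a clicker game, holding coins, bought item counts, cursor damage and total DPS.
; On begin play it sets up Enhanced Input and starts a looping timer that damages the spawned enemy using total DPS.
; Purchases deduct count-based costs, spawn the item, raise cursor damage or DPS scaled by ascension, then refresh UI and check ascension requirements.
; Input events open the pause menu and swap the mouse cursor image.
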(event Custom|UpdateAmountOfCoins
  (params (AmountOfCoins :type Integer) (bAdd :type Boolean))
  ;[1 1 1] Coins: Update Amount
  (bind _output_get (Variables|Default|SetAmountOfCoins (select bAdd (+ AmountOfCoins (Variables|Default|GetAmountOfCoins)) (- AmountOfCoins (Variables|Default|GetAmountOfCoins)))))
  (Default|UpdateCoinsAmountUI (Variables|/Game/Dynamic/Blueprints/BP_IdleMonsterClicker_PC.BP_IdleMonsterClicker_PC_C|GetWB_Main (Variables|Default|GetPlayer%20Controller)) _output_get))

(event Custom|PurchaseItem
  (params (Item :type S%20Item%20Info%20Structure) (ShopItemCard :type WB%20Shop%20Item%20Card%20Object%20Reference))
  (bind (_name _thumbnail _item _dps) (Utilities|Struct|BreakS_ItemInfo Item))
  (bind _itemsbought (Variables|Default|GetItemsBought))
  (bind _value (Utilities|Map|Find _itemsbought _name))
  ;[1 1 1] Item: Purchase
  (Audio|PlaySound2D (Variables|Default|GetSFXPurchase) 1.0 1.0 0.0 0 0)
  (bind _output_get (Variables|Default|SetAmountOfCoins (- (Variables|Default|GetAmountOfCoins) (CallFunction|GetItemCost Item))))
  (Default|UpdateCoinsAmountUI (Variables|/Game/Dynamic/Blueprints/BP_IdleMonsterClicker_PC.BP_IdleMonsterClicker_PC_C|GetWB_Main (Variables|Default|GetPlayer%20Controller)) _output_get)
  (Utilities|Map|Add (Variables|Default|GetItemsBought) _name (+ _value 1))
  (Default|UpdateItemsBoughtUI ShopItemCard)
  (Default|UpdateItemCost ShopItemCard)
  (Default|UpdateShopItemBuyTextColor (Variables|Default|GetPlayer%20Controller))
  (Default|SpawnItem (Variables|Default|GetPlayer%20Controller) (Utilities|Struct|BreakS_ItemInfo Item) (Utilities|Array|Get(acopy) (Default|GetItemSpawnpoint (Variables|Default|GetGame%20Mode) _item) (- _value 0)))
  (if (Utilities|Enum|Equal(Enum) _item "NewEnumerator2")
    (CallFunction|IncreaseCursorDamage (* (Utilities|Struct|BreakS_AscensionMultiplier (CallFunction|GetAscensionDamageMultiplier (Variables|/Game/Dynamic/Blueprints/BP_IdleMonsterClicker_GM.BP_IdleMonsterClicker_GM_C|GetAscensionLevel (Variables|Default|GetGame%20Mode)))) _dps))
    (else
      (CallFunction|UpdateTotalDPS)))
  (Default|UpdateToolTipUI (Variables|/Game/Dynamic/Blueprints/BP_IdleMonsterClicker_PC.BP_IdleMonsterClicker_PC_C|GetShopToolTip (Variables|Default|GetPlayer%20Controller)) Item)
  (Default|CheckAscensionRequirement (Variables|Default|GetGame%20Mode)))

(event Custom|AutoDamage
  ;[1 1 1] Enemy: Auto Damage (Items DPS)
  (bind _returnvalue (Utilities|Time|SetTimerbyFunctionName 0 "AutoDamageFunction" (Variables|Default|GetAutoDamageTimerTime) true))
  (Variables|Default|SetAutoDamageHandle _returnvalue))

(event Input|EnhancedActionEvents|EnhancedInputActionIA_MouseClicking
  (params (ActionValue :type Boolean) (ElapsedSeconds :type Float%20%28double-precision%29) (TriggeredSeconds :type Float%20%28double-precision%29) (InputAction :type Input%20Action%20Object%20Reference :default "/Game/Dynamic/Blueprints/Player/Input/IA_MouseClicking.IA_MouseClicking"))
  (bind _player_controller (Variables|Default|GetPlayer%20Controller))
  (bind _mousecursor (Variables|/Game/Dynamic/Blueprints/BP_IdleMonsterClicker_PC.BP_IdleMonsterClicker_PC_C|GetMouseCursor _player_controller))
  ;[1 1 1] Game: Mouse Input | Mouse States
  (:Triggered
    (Default|SetMouseCursorImage _mousecursor "NewEnumerator1"))
  (:Completed
    (Default|SetMouseCursorImage _mousecursor "NewEnumerator0")))

(event Input|EnhancedActionEvents|EnhancedInputActionIA_PauseMenu
  (params (ActionValue :type Boolean) (ElapsedSeconds :type Float%20%28double-precision%29) (TriggeredSeconds :type Float%20%28double-precision%29) (InputAction :type Input%20Action%20Object%20Reference :default "/Game/Dynamic/Blueprints/Player/Input/IA_PauseMenu.IA_PauseMenu"))
  ;[1 1 1] Input: Pause Menu
  (:Started
    (bind _returnvalue (UserInterface|CreateWidget "/Game/Dynamic/UI/WB_PauseMenu.WB_PauseMenu_C"))
    (UserInterface|Viewport|AddtoViewport _returnvalue 0)
    (Input|SetInputModeUIOnly (Game|GetPlayerController 0) 0 "DoNotLock" false)
    (Game|SetGamePaused true)))

(event EventBeginPlay
  ;[1 1 1] Game: Begin Play
  (bind _playercontroller (Class|BPIPlayerController|GetPlayerControlRef(Message) (Game|GetPlayerController 0)))
  (Variables|Default|SetPlayer%20Controller _playercontroller)
  (bind _gamemode (Class|BPIGameMode|GetGameModeRef(Message) (Game|GetGameMode)))
  (Variables|Default|SetGame%20Mode _gamemode)
  (Utilities|IsValid (PlayerController|LocalPlayerSubsystems|GetEnhancedInputLocalPlayerSubsystem (Variables|Default|GetPlayer%20Controller))
    (:Is%20Valid
      (Input|AddMappingContext (PlayerController|LocalPlayerSubsystems|GetEnhancedInputLocalPlayerSubsystem (Variables|Default|GetPlayer%20Controller)) "/Game/Dynamic/Blueprints/Player/Input/IMC_Default.IMC_Default" 0 "(bIgnoreAllPressedKeysUntilRelease=True,bForceImmediately=False,bNotifyUserSettings=False)")
      (Utilities|IsValid (Variables|/Game/Dynamic/Blueprints/BP_IdleMonsterClicker_PC.BP_IdleMonsterClicker_PC_C|GetWB_Main (Variables|Default|GetPlayer%20Controller))
        (:Is%20Valid
          (Default|UpdateCoinsAmountUI (Variables|/Game/Dynamic/Blueprints/BP_IdleMonsterClicker_PC.BP_IdleMonsterClicker_PC_C|GetWB_Main (Variables|Default|GetPlayer%20Controller)) (Variables|Default|GetAmountOfCoins))
          (CallFunction|AutoDamage))))))

(fn ConstructionScript)

(fn DoesPlayerHaveEnoughCoins
  (params (ItemCost :type Integer))
  (return (>= (Variables|Default|GetAmountOfCoins) ItemCost)))

(fn GetItemCost
  (params (S_ItemInfo :type S%20Item%20Info%20Structure%20%28by%20ref%29))
  (bind (_name _thumbnail _item) (Utilities|Struct|BreakS_ItemInfo S_ItemInfo))
  (bind _itemsbought (Variables|Default|GetItemsBought))
  (bind _value (Utilities|Map|Find _itemsbought _name))
  (bind _itemcostinfo (CallFunction|GetItemCost _value))
  (bind (_lightfeather _torch _cursor _luckyrainbow _orcskull _knighthelmet _grandwizardhat _crownofevil _kingscrown _theprotector _runeoftime) (Utilities|Struct|BreakS_ItemCost _itemcostinfo))
  (return (Utilities|Select :Index _item :NewEnumerator2 _cursor :NewEnumerator0 _lightfeather :NewEnumerator1 _torch :NewEnumerator3 _luckyrainbow :NewEnumerator4 _orcskull :NewEnumerator5 _knighthelmet :NewEnumerator6 _grandwizardhat :NewEnumerator7 _crownofevil :NewEnumerator8 _kingscrown :NewEnumerator9 _theprotector :NewEnumerator10 _runeoftime)))

(fn AutoDamageFunction
  (Game|Damage|ApplyDamage (Variables|/Game/Dynamic/Blueprints/BP_IdleMonsterClicker_PC.BP_IdleMonsterClicker_PC_C|GetSpawnedEnemy (Variables|Default|GetPlayer%20Controller)) (/ (Variables|Default|GetTotalDPS) (/ 1.0 (Variables|Default|GetAutoDamageTimerTime))) 0 0 "/Game/Dynamic/Blueprints/BP_AutoDamage.BP_AutoDamage_C"))

(fn UpdateTotalDPS
  (bind _keys (Utilities|Map|Keys (Variables|Default|GetItemsBought)))
  (for (_array_element _array_index) _keys
    (if (Utilities|Enum|NotEqual(Enum) (.Item (Utilities|Struct|BreakS_ItemInfo (CallFunction|GetItemInfo _array_element))) "NewEnumerator2")
      (bind _values (Utilities|Map|Values (Variables|Default|GetItemsBought)))
      (Variables|Default|SetTotalDPS (+ (Variables|Default|GetTotalDPS) (* (Utilities|Array|Get(acopy) _values _array_index) (* (.DPS (Utilities|Struct|BreakS_ItemInfo (CallFunction|GetItemInfo _array_element))) (Utilities|Struct|BreakS_AscensionMultiplier (CallFunction|GetAscensionDamageMultiplier (Variables|/Game/Dynamic/Blueprints/BP_IdleMonsterClicker_GM.BP_IdleMonsterClicker_GM_C|GetAscensionLevel (Variables|Default|GetGame%20Mode))))))))))
  (Variables|Default|SetTotalDPS (Variables|Default|GetTotalDPS)))

(fn IncreaseCursorDamage
  (params (DamageToAdd :type Float%20%28double-precision%29))
  (Variables|Default|SetCursorDamage (+ DamageToAdd (Variables|Default|GetCursorDamage))))

(fn GetPlayerRef
  (return self))