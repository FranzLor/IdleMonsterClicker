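; Game mode for an idle monster clicker that runs level progression, the timed enemy fight and ascension resets.
; Level data picks the enemy the player controller spawns, and a looping timer restores its health when time runs out.
; BP_ItemSpawn markers expand into per-item grids of spawn positions.
; Owning every shop item reveals the ascension UI, and restarting raises the ascension level while resetting levels, coins, items and damage.
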(event Custom|UnlockLevel
  (if (== (Variables|Default|GetCurrentLevel) (Variables|Default|GetUnlockedLevel))
    (bind _result (Math|Integer|IncrementInt (Variables|Default|GetUnlockedLevel))
      (:%20%20
        (if (<= _result (Variables|Default|GetMaxLevel))
          (Default|AddLevelButtonUI (Variables|Default|GetPlayer%20Controller) (Variables|Default|GetUnlockedLevel))
          (Audio|PlaySound2D (Utilities|Select :Index (.EnemyType (Utilities|Struct|BreakS_Enemy (CallFunction|GetEnemyInfo (Utilities|Struct|BreakS_LevelInfo (CallFunction|GetLevelInfo (Variables|Default|GetUnlockedLevel)))))) :NewEnumerator0 (Variables|Default|GetSFXLevelUnlockNormal) :NewEnumerator1 (Variables|Default|GetSFXLevelUnlockBoss)) 1.0 1.0 0.0 0 0))))))

(event Custom|SetCurrentLevel
  (params (Level :type Integer))
  (bind (_enemy _spawntransform) (CallFunction|GetEnemytoSpawnonCurrentLevel))
  (Variables|Default|SetCurrentLevel Level)
  (bind _spawnedenemy (Variables|/Game/Dynamic/Blueprints/BP_IdleMonsterClicker_PC.BP_IdleMonsterClicker_PC_C|GetSpawnedEnemy (Variables|Default|GetPlayer%20Controller))
    (:then
      (Actor|DestroyActor _spawnedenemy))
    (:else
      _))
  (Default|SpawnEnemy (Variables|Default|GetPlayer%20Controller) _enemy _spawntransform)
  (CallFunction|StartRoundTimer))

(event Custom|RoundTimerLoop
  (bind _output_get (Variables|Default|SetCurrentRoundTimer (Math|Float|Clamp(Float) (- (Variables|Default|GetCurrentRoundTimer) (Variables|Default|GetRoundTImerTIme)) 0.0 (Variables|Default|GetCurrentRoundTimer))))
  (Default|UpdateTimerUI (Variables|/Game/Dynamic/Blueprints/BP_IdleMonsterClicker_PC.BP_IdleMonsterClicker_PC_C|GetWB_Main (Variables|Default|GetPlayer%20Controller)) _output_get)
  (if (== (Variables|Default|GetCurrentRoundTimer) 0.0)
    (Default|RestoreHealth (Variables|/Game/Dynamic/Blueprints/BP_IdleMonsterClicker_PC.BP_IdleMonsterClicker_PC_C|GetSpawnedEnemy (Variables|Default|GetPlayer%20Controller)))
    (Variables|Default|SetCurrentRoundTimer (Variables|Default|GetInitialRoundTimer))))

(event Custom|StartRoundTimer
  (Variables|Default|SetCurrentRoundTimer (Variables|Default|GetInitialRoundTimer))
  (bind _returnvalue (Utilities|Time|SetTimerbyEvent (delegate Custom|RoundTimerLoop) (Variables|Default|GetRoundTImerTIme) true))
  (Variables|Default|SetRoundTimerHandling _returnvalue))

(event Custom|RestartGame
  (bind _playerpawn (Variables|Default|GetPlayerPawn))
  (bind _player_controller (Variables|Default|GetPlayer%20Controller))
  (Math|Integer|IncrementInt (Variables|Default|GetAscensionLevel)
    (:%20%20
      (Variables|Default|SetAscensionRequirementMet false)
      (Variables|Default|SetUnlockedLevel 1)
      (Variables|Default|SetCurrentLevel 1)
      (Widget|Panel|ClearChildren (Variables|/Game/Dynamic/UI/WB_MainUI.WB_MainUI_C|GetVB_LevelList (Variables|/Game/Dynamic/Blueprints/BP_IdleMonsterClicker_PC.BP_IdleMonsterClicker_PC_C|GetWB_Main _player_controller)))
      (Default|AddLevelButtonUI _player_controller (Variables|Default|GetUnlockedLevel))
      (bind _output_get (Variables|/Game/Dynamic/Blueprints/Player/BP_Player.BP_Player_C|SetAmountOfCoins (Variables|Default|GetPlayerPawn) 0))
      (Default|UpdateCoinsAmountUI (Variables|/Game/Dynamic/Blueprints/BP_IdleMonsterClicker_PC.BP_IdleMonsterClicker_PC_C|GetWB_Main (Variables|Default|GetPlayer%20Controller)) _output_get)
      (Utilities|Map|Clear (Variables|/Game/Dynamic/Blueprints/Player/BP_Player.BP_Player_C|GetItemsBought (Variables|Default|GetPlayerPawn)))
      (Default|CreateShopItemCards (Variables|Default|GetPlayer%20Controller))
      (Variables|/Game/Dynamic/Blueprints/Player/BP_Player.BP_Player_C|SetTotalDPS _playerpawn 0.0)
      (Variables|/Game/Dynamic/Blueprints/Player/BP_Player.BP_Player_C|SetCursorDamage _playerpawn 1e+01)
      (CallFunction|SetCurrentLevel (Variables|Default|GetCurrentLevel)))))

(event EventBeginPlay
  (bind (_enemy _spawntransform) (CallFunction|GetEnemytoSpawnonCurrentLevel))
  (bind _returnvalue (Actor|GetActorOfClass "/Game/Dynamic/Blueprints/Spawnpoints/BP_EnemySpawn.BP_EnemySpawn_C"))
  (Variables|Default|SetEnemySpawn _returnvalue)
  (bind _playercontroller (Class|BPIPlayerController|GetPlayerControlRef(Message) (Game|GetPlayerController 0)))
  (bind _output_get (Variables|Default|SetPlayer%20Controller _playercontroller))
  (bind _player (Class|BPIPlayer|GetPlayerRef(Message) (Game|GetPlayerCharacter 0)))
  (Variables|Default|SetPlayerPawn _player)
  (CallFunction|SetItemSpawnpoints)
  (bind _outrownames (DataTable|GetDataTableRowNames "/Game/Dynamic/Blueprints/DataTables/DT_ItemInfo.DT_ItemInfo"))
  (Variables|Default|SetAmountOfShopItems (Utilities|Array|Length _outrownames))
  (Default|SpawnEnemy _output_get _enemy _spawntransform)
  (CallFunction|StartRoundTimer))

(fn ConstructionScript)

(fn GetEnemytoSpawnonCurrentLevel
  (return (.Class (Utilities|Struct|BreakS_Enemy (CallFunction|GetEnemyInfo (Utilities|Struct|BreakS_LevelInfo (CallFunction|GetLevelInfo (Variables|Default|GetCurrentLevel)))))) (Transformation|GetActorTransform (Variables|Default|GetEnemySpawn))))

(fn GetEnemySpawn
  (return (.Class (Utilities|Struct|BreakS_Enemy (CallFunction|GetEnemyInfo (Utilities|Struct|BreakS_LevelInfo (CallFunction|GetLevelInfo (Variables|Default|GetCurrentLevel)))))) (Transformation|GetActorTransform (Variables|Default|GetEnemySpawn))))

(fn SetItemSpawnpoints
  (bind _outactors (Actor|GetAllActorsOfClass "/Game/Dynamic/Blueprints/Spawnpoints/BP_ItemSpawn.BP_ItemSpawn_C"))
  (bind _output_get (LocalVariables|SetLocalItemSpawnpoints _outactors))
  (if (> (Utilities|Array|Length _output_get) 0)
    (for _index (range 0 (LocalVariables|GetLocalLoopLastIndex)) :!label _label
      (Utilities|Array|Add (Utilities|Select :Index (Variables|/Game/Dynamic/Blueprints/Spawnpoints/BP_ItemSpawn.BP_ItemSpawn_C|GetItem (Utilities|Array|Get(acopy) (LocalVariables|GetLocalItemSpawnpoints))) :NewEnumerator2 (Variables|Default|GetCursor) :NewEnumerator0 (Variables|Default|GetLightFeatherSpawnpoints) :NewEnumerator1 (Variables|Default|GetTorchSpawnpoint) :NewEnumerator3 (Variables|Default|GetLuckyRainbow) :NewEnumerator4 (Variables|Default|GetOrcSkull) :NewEnumerator5 (Variables|Default|GetKnightHelmet) :NewEnumerator6 (Variables|Default|GetGrandWizardHat) :NewEnumerator7 (Variables|Default|GetCrownOfEvil) :NewEnumerator8 (Variables|Default|GetKingsCrown) :NewEnumerator9 (Variables|Default|GetTheProtector) :NewEnumerator10 (Variables|Default|GetRuneOfTime)) (Math|Vector|MakeVector (+ (.X (Math|Vector|BreakVector (Transformation|GetActorLocation (Utilities|Array|Get(acopy) (LocalVariables|GetLocalItemSpawnpoints))))) (* 1e+01 _index)) (.Y (Math|Vector|BreakVector (Transformation|GetActorLocation (Utilities|Array|Get(acopy) (LocalVariables|GetLocalItemSpawnpoints))))) (- (.Z (Math|Vector|BreakVector (Transformation|GetActorLocation (Utilities|Array|Get(acopy) (LocalVariables|GetLocalItemSpawnpoints))))) (* 1e+01 (LocalVariables|GetLocalZAxisMultiplier)))))
      (if (== (LocalVariables|GetLocalLoopLastIndex) _index)
        (bind _result (Math|Integer|IncrementInt (LocalVariables|GetLocalLoopCounter))
          (:%20%20
            (if (< _result (LocalVariables|GetLocalAmountOfRows))
              (Math|Integer|IncrementInt (LocalVariables|GetLocalZAxisMultiplier)
                (:%20%20
                  (goto _label)))
              (else
                (Utilities|Array|RemoveIndex (LocalVariables|GetLocalItemSpawnpoints))
                (if (Utilities|Array|IsNotEmpty (LocalVariables|GetLocalItemSpawnpoints))
                  (LocalVariables|SetLocalZAxisMultiplier 0)
                  (LocalVariables|SetLocalLoopCounter 0)
                  (goto _label))))))))))

(fn GetItemSpawnpoint
  (params (ItemName :type E_Items%20Enum :default "NewEnumerator0"))
  (switch Utilities|FlowControl|Switch|SwitchonE_Items ItemName
    (:NewEnumerator2
      (return (Variables|Default|GetCursor)))
    (:NewEnumerator0
      (return (Variables|Default|GetLightFeatherSpawnpoints)))
    (:NewEnumerator1
      (return (Variables|Default|GetTorchSpawnpoint)))
    (:NewEnumerator3
      (return (Variables|Default|GetLuckyRainbow)))
    (:NewEnumerator4
      (return (Variables|Default|GetOrcSkull)))
    (:NewEnumerator5
      (return (Variables|Default|GetKnightHelmet)))
    (:NewEnumerator6
      (return (Variables|Default|GetGrandWizardHat)))
    (:NewEnumerator7
      (return (Variables|Default|GetCrownOfEvil)))
    (:NewEnumerator8
      (return (Variables|Default|GetKingsCrown)))
    (:NewEnumerator9
      (return (Variables|Default|GetTheProtector)))
    (:NewEnumerator10
      (return (Variables|Default|GetRuneOfTime)))))

(fn CheckAscensionRequirement
  (if (not (Variables|Default|GetAscensionRequirementMet))
    (bind _keys (Utilities|Map|Keys (Variables|/Game/Dynamic/Blueprints/Player/BP_Player.BP_Player_C|GetItemsBought (Variables|Default|GetPlayerPawn))))
    (if (== (Utilities|Array|Length _keys) (Variables|Default|GetAmountOfShopItems))
      (bind _values (Utilities|Map|Values (Variables|/Game/Dynamic/Blueprints/Player/BP_Player.BP_Player_C|GetItemsBought (Variables|Default|GetPlayerPawn))))
      (bind _array_element (Utilities|Array|ForEachLoopwithBreak _values :!label _label)
        (:LoopBody
          (if (>= _array_element 1)
            (Math|Integer|IncrementInt (LocalVariables|GetLocalCounter))
            (else
              (goto _label Break))))
        (:Completed
          (if (== (LocalVariables|GetLocalCounter) (Variables|Default|GetAmountOfShopItems))
            (Variables|Default|SetAscensionRequirementMet true)
            (Widget|SetVisibility (Variables|/Game/Dynamic/UI/WB_MainUI.WB_MainUI_C|GetOV_Ascension (Variables|/Game/Dynamic/Blueprints/BP_IdleMonsterClicker_PC.BP_IdleMonsterClicker_PC_C|GetWB_Main (Variables|Default|GetPlayer%20Controller))) "SelfHitTestInvisible")))))))

(fn GetGameModeRef
  (return self))